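; BPDamageCube is an actor that damages a BPCharacter when it overlaps one.
; Each overlap begin stores the cast character, subtracts one Health, passes the new value to the character's Gamemode through UpdateHealth and prints a debug message.
; The character is destroyed only when Health equals exactly zero.
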(event `self.ReceiveActorBeginOverlap`
  (params (OtherActor :type "Actor Object Reference"))
  (bind _asbpcharacter (cast `/Game/Blueprints/Characters/BPCharacter` OtherActor))
  (bind _output_get (set `self.Character` _asbpcharacter))
  (bind _output_get_2 (set `/Game/Blueprints/Characters/BPCharacter.Health` (- (`/Game/Blueprints/Characters/BPCharacter.Health` _asbpcharacter) 1.0) _output_get))
  (`/Game/Blueprints/Gamemodes/BPGamemode.UpdateHealth` (`/Game/Blueprints/Characters/BPCharacter.Gamemode` (`self.Character`)) _output_get_2)
  (`KismetSystemLibrary.PrintString` "Damaged" true true (struct :`R` 1.0 :`A` 1.0))
  (if (== (`/Game/Blueprints/Characters/BPCharacter.Health` (`self.Character`)) 0.0)
    (`self.K2_DestroyActor` (`self.Character`))))

(fn `UserConstructionScript`)
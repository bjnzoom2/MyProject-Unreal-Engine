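; Bullet projectile actor that launches itself on spawn and destroys itself on overlap.
; On BeginPlay it takes the right vector of the static mesh's socket rotation, prints it, and applies it as a velocity-change impulse to the mesh, so movement relies on physics.
; Any actor overlap destroys the bullet, with no damage or hit handling.
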(event `self.ReceiveBeginPlay`
  (bind _output_get (set `self.ForwardVector` (`KismetMathLibrary.GetRightVector` (`SceneComponent.GetSocketRotation` (`self.StaticMesh`) "None"))))
  (`KismetSystemLibrary.PrintString` (`KismetStringLibrary.Conv_VectorToString` _output_get))
  (`PrimitiveComponent.AddImpulse` (`self.StaticMesh`) (* (`self.ForwardVector`) (2500.0 2500.0 2500.0)) "None" true))

(event `self.ReceiveActorBeginOverlap`
  (params (OtherActor :type "Actor Object Reference"))
  (`self.K2_DestroyActor`))

(event `self.ReceiveTick`
  (params (DeltaSeconds :type "Float (single-precision)")))

(fn `UserConstructionScript`)
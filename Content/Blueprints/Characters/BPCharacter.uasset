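; BPCharacter is a player-controllable character that can move, look around and spawn actors.
; Axis inputs drive movement along the actor's forward and right vectors, plus controller yaw and pitch.
; Pressing Create spawns a BPActor offset along the mesh's right vector, using an unnamed socket as origin and adjusting for collisions but always spawning.
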(event `InputAxis|MoveAlongForwardVector`
  (params (AxisValue :type "Float (single-precision)"))
  ;[1 1 1] Movement And Camera
  (`self.AddMovementInput` (`self.GetActorForwardVector`) AxisValue))

(event `InputAxis|MoveAlongRightVector`
  (params (AxisValue :type "Float (single-precision)"))
  ;[1 1 1] Movement And Camera
  (`self.AddMovementInput` (`self.GetActorRightVector`) AxisValue))

(event `InputAxis|LookAround`
  (params (AxisValue :type "Float (single-precision)"))
  ;[1 1 1] Movement And Camera
  (`self.AddControllerYawInput` AxisValue))

(event `InputAxis|LookUpward`
  (params (AxisValue :type "Float (single-precision)"))
  ;[1 1 1] Movement And Camera
  (`self.AddControllerPitchInput` AxisValue))

(event `InputAction|Create`
  (params (Key :type "Key Structure"))
  (bind _mesh (`self.Mesh`))
  (:`Pressed`
    (`|SpawnActorFromClass` "/Game/Blueprints/Actors/BPActor.BPActor_C" (`KismetMathLibrary.Conv_VectorToTransform` (+ (`SceneComponent.GetSocketLocation` _mesh "None") (* (`KismetMathLibrary.GetRightVector` (`SceneComponent.GetSocketRotation` _mesh "None")) (200.0 200.0 200.0)))) "AdjustIfPossibleButAlwaysSpawn" "MultiplyWithRoot" null null)))

(fn `UserConstructionScript`)
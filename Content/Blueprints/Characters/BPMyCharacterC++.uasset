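; Player character Blueprint on a C++ base, forwarding input to inherited movement, camera, dash, fly/jump and "Solver" ability functions.
; BeginPlay hands the camera, spring arm, solver mesh, yellow outline and shape meshes to the base class variables.
; Solver inputs handle activation, mesh use, editing and mode switching, with SolverUse running every Tick and the outline passed into targeting.
; Landing re-enables dashing.
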(event `self.ReceiveBeginPlay`
  (set `self.cameraComp` (`self.Camera`))
  (set `self.springArmComp` (`self.SpringArm`))
  (set `self.solverMeshComp` (`self.SolverMesh`))
  (set `self.Outline` "/Game/Materials/Outlines/YellowOutline.YellowOutline")
  (set `self.shapeMeshes` (`self.shapeMeshes`)))

(event `self.ReceiveActorBeginOverlap`
  (params (OtherActor :type "Actor Object Reference")))

(event `self.OnLanded`
  (params (Hit :type "HitResult Structure (by ref)"))
  (set `self.bCanDash` true))

(event `InputAxis|MoveAlongForwardVector`
  (params (AxisValue :type "Float (single-precision)"))
  ;[1 1 1] Movement And Camera
  (`self.MoveAlongForwardVector` AxisValue))

(event `Key|SpaceBar`
  (params (Key :type "Key Structure"))
  ;[1 1 1] Movement And Camera
  (:`Pressed`
    (`self.Fly`)
    (`self.Jump`)))

(event `InputAxis|MoveAlongRightVector`
  (params (AxisValue :type "Float (single-precision)"))
  ;[1 1 1] Movement And Camera
  (`self.MoveAlongRightVector` AxisValue))

(event `InputAxis|MoveAlongUpVector`
  (params (AxisValue :type "Float (single-precision)"))
  ;[1 1 1] Movement And Camera
  (`self.MoveAlongUpVector` AxisValue))

(event `InputAxis|LookAround`
  (params (AxisValue :type "Float (single-precision)"))
  ;[1 1 1] Movement And Camera
  (`self.LookAround` AxisValue))

(event `InputAction|Dash`
  (params (Key :type "Key Structure"))
  ;[1 1 1] Movement And Camera
  (:`Pressed`
    (`self.Dash`)))

(event `InputAxis|LookUpward`
  (params (AxisValue :type "Float (single-precision)"))
  ;[1 1 1] Movement And Camera
  (`self.LookUp` AxisValue))

(event `InputAction|Shoot`
  (params (Key :type "Key Structure"))
  ;[1 1 1] Actions
  (:`Pressed`
    (`self.GetOtherActor` (`self.Outline`))))

(event `InputAction|UseSolver`
  (params (Key :type "Key Structure"))
  ;[1 1 1] Actions
  (:`Pressed`
    (`self.SolverUseMesh` (`self.Outline`))))

(event `InputAction|SolverActivation`
  (params (Key :type "Key Structure"))
  ;[1 1 1] Actions
  (:`Pressed`
    (`self.ActivateSolver`)))

(event `InputAction|SolverEditMode`
  (params (Key :type "Key Structure"))
  ;[1 1 1] Actions
  (:`Pressed`
    (`self.SolverEdit` Key)))

(event `InputAction|SwitchSolverMode`
  (params (Key :type "Key Structure"))
  ;[1 1 1] Actions
  (:`Pressed`
    (`self.SwitchSolverMode` (`self.GetInputAxisKeyValue` Key))
    (`KismetSystemLibrary.PrintString` (`|GetEnumeratorNameAsString` (`self.solverMode`)))))

(event `self.ReceiveTick`
  (params (DeltaSeconds :type "Float (single-precision)"))
  (`self.SolverUse`))

(fn `UserConstructionScript`)
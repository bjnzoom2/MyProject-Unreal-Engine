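; BPController is a controller Blueprint that shows or hides the solver edit HUD based on the player character's solver mode.
; On BeginPlay it caches the BPMyCharacter actor and creates the BP_HUD_Solver_Edit widget.
; Every Tick it polls SolverMode, calling AddToViewport in one specific mode and RemoveFromParent otherwise, without checking whether the widget's visibility needs changing.
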(event `self.ReceiveBeginPlay`
  (bind _returnvalue (`GameplayStatics.GetActorOfClass` "/Game/Blueprints/Characters/BPMyCharacterC++.BPMyCharacterC++_C"))
  (set `self.PlayerCharacter` _returnvalue)
  (bind _returnvalue_2 (`|CreateWidget` "/Game/Blueprints/UI/HUD/BP_HUD_Solver_Edit.BP_HUD_Solver_Edit_C"))
  (set `self.SolverHUD` _returnvalue_2))

(event `self.ReceiveTick`
  (params (DeltaSeconds :type "Float (single-precision)"))
  (`self.SolverEditHUD`))

(event `SolverEditHUD`
  (bind _solverhud (`self.SolverHUD`))
  (`self.SolverHUD`
    (:`then`
      (if (== (`MyCharacter.solverMode` (`self.PlayerCharacter`)) 3)
        (`UserWidget.AddToViewport` _solverhud 0)
        (else
          (`Widget.RemoveFromParent` _solverhud))))
    (:`else`)))

(fn `UserConstructionScript`)